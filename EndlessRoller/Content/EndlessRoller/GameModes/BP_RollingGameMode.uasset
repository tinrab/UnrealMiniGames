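; Game mode for an endless roller that keeps generating track by chaining randomly chosen platforms.
; BeginPlay spawns an initial batch, each placed at the previous platform's attachment transform.
; When the player reaches a platform's end, another spawns and the oldest passed platform is destroyed once their count hits the limit.
; SpawnPlatform picks classes using density weights, though its "cumulative" values sum only adjacent pairs.
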(event `self.ReceiveBeginPlay`
  (for _ (range (+ (`self.MaxSpawnedPlatforms`) 1))
    (bind _platform (`self.SpawnPlatform` :!label _label))
    (add `/Game/EndlessRoller/Environment/BP_Platform.OnPlayerEndReached` _platform (delegate `Event PlayerEndReached`))))

(event `Event PlayerEndReached`
  (params (Platform :type "/Game/EndlessRoller/Environment/BP_Platform Object Reference"))
  (bind _spawnedplatforms (`self.SpawnedPlatforms`))
  (bind _spawnedplatforms_2 (`self.SpawnedPlatforms`))
  (remove `/Game/EndlessRoller/Environment/BP_Platform.OnPlayerEndReached` Platform (delegate `Event PlayerEndReached`))
  (`|ExecutionSequence`
    (:`then_0`
      ;[1 1 1] Limit number of platforms
      (`KismetArrayLibrary.Array_Add` _spawnedplatforms Platform)
      (if (>= (`KismetArrayLibrary.Array_Length` _spawnedplatforms) (`self.MaxSpawnedPlatforms`))
        ;[1 1 1] Destroy platform
        (`self.K2_DestroyActor` (`|GetArrayItem` _spawnedplatforms_2))
        (`KismetArrayLibrary.Array_Remove` _spawnedplatforms_2)))
    (:`then_1`
      (goto _label))))

(fn `SpawnPlatform`
  (returns (Platform :type "/Game/EndlessRoller/Environment/BP_Platform Object Reference"))
  (locals (Densities :type "Array of Float (double-precision)") (Platforms :type "Array of /Game/EndlessRoller/Environment/BP_Platform Class Reference") (CumulativeDensities :type "Array of Float (double-precision)") (RandomValue :type "Float (double-precision)") (SelectedPlatform :type "/Game/EndlessRoller/Environment/BP_Platform Class Reference" :default null))
  (bind _densities (`local.Densities`))
  (bind _cumulativedensities (`local.CumulativeDensities`))
  ;[1 1 1] Compute cumulative densities
  (`KismetArrayLibrary.Array_Add` (`local.CumulativeDensities`) (`|GetArrayItem` (`local.Densities`)))
  (for _index (range 1 (+ (`KismetArrayLibrary.Array_LastIndex` (`local.Densities`)) 1))
    (`KismetArrayLibrary.Array_Add` (`local.CumulativeDensities`) (+ (`|GetArrayItem` _densities _index) (`|GetArrayItem` _densities (- _index 1)))))
  (set `local.RandomValue` (`KismetMathLibrary.RandomFloatInRange` 0.0 (`|GetArrayItem` _cumulativedensities (`KismetArrayLibrary.Array_LastIndex` _cumulativedensities))))
  ;[1 1 1] Select platform class
  (for (_array_element _array_index) (`local.Platforms`)
    (if (>= (`|GetArrayItem` (`local.CumulativeDensities`) _array_index) (`local.RandomValue`))
      (set `local.SelectedPlatform` _array_element)
      (break)))
  ;[1 1 1] Spawn platform
  (bind _returnvalue (`|SpawnActorFromClass` (`local.SelectedPlatform`) (`self.NextAttachment`) "Undefined" "OverrideRootScale" null null))
  (set `self.NextAttachment` (`/Game/EndlessRoller/Environment/BP_Platform.GetAttachment` _returnvalue))
  (return _returnvalue))

(fn `UserConstructionScript`)